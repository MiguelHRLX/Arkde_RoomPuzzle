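; Player character Blueprint with a selectable first- or third-person camera and debug feedback for an ultimate ability.
; BeginPlay adds the BP_Sight widget to the viewport.
; The construction script uses UseFirstPersonView to choose which camera auto-activates.
; Ultimate events for XP gain, start, stop and duration updates only print colored on-screen messages, with XP text color reflecting whether the ultimate is usable.
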(event EventBeginPlay
  (bind _returnvalue (UserInterface|CreateWidget "/Game/Widgets/BP_Sight.BP_Sight_C"))
  (UserInterface|Viewport|AddtoViewport _returnvalue 0))

(event Collision|EventActorBeginOverlap
  (params (OtherActor :type Actor%20Object%20Reference)))

(event EventTick
  (params (DeltaSeconds :type Float%20%28single-precision%29)))

(event EventStartUltimate
  (Development|PrintString "start Ultimate" true true "(R=1.000000,G=0.106739,B=0.000000,A=1.000000)"))

(event EventGainUltimateXP
  (params (XPGained :type Float%20%28single-precision%29))
  (Development|PrintString (Utilities|String|Append "XP gain" (Utilities|String|ToString(Float) XPGained) "|| Ultimate  XP" (Utilities|String|ToString(Float) (Variables|Default|GetCurrentUltimateXP)) "/" (Utilities|String|ToString(Float) (Variables|Default|GetMaxUltimateXP))) true true (select (Variables|Default|GetbCanUseUltimate) "(R=0.309646,G=1.000000,B=0.000000,A=1.000000)" "(R=0.004949,G=0.288888,B=1.000000,A=1.000000)") 5.0))

(event EventStopUltimate
  (Development|PrintString "Stop Ultimate" true true "(R=1.000000,G=0.049283,B=0.960843,A=1.000000)"))

(event EventUpdateUltimateDuration
  (params (value :type Float%20%28single-precision%29))
  (Development|PrintString (Utilities|String|Append (Utilities|String|ToString(Float) (Variables|Default|GetCurrentUltimateDuration)) "/" (Utilities|String|ToString(Float) (Variables|Default|GetMaxUltimateDuration))) true true "(R=1.000000,G=0.000000,B=0.066736,A=1.000000)"))

(fn ConstructionScript
  (Components|Activation|SetAutoActivate (Variables|Default|GetFPSCameraComponent) (Variables|Default|GetbUseFirstPersonView))
  (Components|Activation|SetAutoActivate (Variables|Default|GetTPSCameraComponent) (not (Variables|Default|GetbUseFirstPersonView))))